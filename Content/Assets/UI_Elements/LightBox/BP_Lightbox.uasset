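; BP_Lightbox is an interactable light box actor that opens a wire minigame for the player.
; A Box overlap with HauntedEscapeCharacter sets PlayerInRange, which is never cleared in this Blueprint.
; Pressing E while that flag is set creates WBP_WireMinigame, adds it to the viewport, switches to UI-only input and shows the mouse cursor.
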(event `self.Box.OnComponentBeginOverlap`
  (params (OverlappedComponent :type "PrimitiveComponent Object Reference") (OtherActor :type "Actor Object Reference") (OtherComp :type "PrimitiveComponent Object Reference") (OtherBodyIndex :type Integer) (bFromSweep :type Boolean) (SweepResult :type "HitResult Structure (by ref)"))
  (cast `HauntedEscapeCharacter` OtherActor)
  (set `self.bPlayerInRange` true))

(event `Key|E`
  (params (Key :type "Key Structure"))
  (:`Pressed`
    (if (`self.bPlayerInRange`)
      (bind _returnvalue (`|CreateWidget` "/Game/Assets/UI_Elements/LightBox/WBP_WireMinigame.WBP_WireMinigame_C"))
      (`UserWidget.AddToViewport` _returnvalue 0)
      (`WidgetBlueprintLibrary.SetInputMode_UIOnlyEx` (`GameplayStatics.GetPlayerController` 0) null)
      (set `PlayerController.bShowMouseCursor` true (`GameplayStatics.GetPlayerController` 0)))))

(fn `UserConstructionScript`)